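; BP_MagicDamageProjectile is a magic projectile that homes in on an assigned actor and damages it.
; SetHomingTarget stores the target and, if it has a capsule component, makes that the ProjectileMovement homing target.
; Sphere overlaps ignore every other actor.
; On reaching a BP_BaseCharacter target, it applies DamageAmount through that character's BPCHealth component and destroys itself.
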(event `SetHomingTarget`
  (params (HomingTarget :type "Actor Object Reference"))
  (bind _returnvalue (`self.GetComponentByClass` HomingTarget "/Script/Engine.CapsuleComponent"))
  (bind _projectilemovement (`self.ProjectileMovement`))
  ;[1 1 1] Make it a homing projectile and set the homing target
  (set `self.HomingTarget` HomingTarget)
  (`/Engine/EditorBlueprintResources/StandardMacros.IsValid` _returnvalue
    (:`Is Valid`
      (set `ProjectileMovementComponent.HomingTargetComponent` _returnvalue _projectilemovement)
      (set `ProjectileMovementComponent.bIsHomingProjectile` true _projectilemovement))))

(event `self.Sphere.OnComponentBeginOverlap`
  (params (OverlappedComponent :type "PrimitiveComponent Object Reference") (OtherActor :type "Actor Object Reference") (OtherComp :type "PrimitiveComponent Object Reference") (OtherBodyIndex :type Integer) (bFromSweep :type Boolean) (SweepResult :type "HitResult Structure (by ref)"))
  (bind _homingtarget (`self.HomingTarget`))
  ;[1 1 1] If you hit the homing target
  (`/Engine/EditorBlueprintResources/StandardMacros.IsValid` OtherActor
    (:`Is Valid`
      (`/Engine/EditorBlueprintResources/StandardMacros.IsValid` _homingtarget
        (:`Is Valid`
          (if (== OtherActor _homingtarget)
            ;[1 1 1] Cast it to base character apply damage and destroy yourself
            (bind _asbp_base_character (cast `/Game/Blueprints/BP_BaseCharacter` (`self.HomingTarget`)))
            (`/Game/Blueprints/BPC_Health.Do Damage` (`/Game/Blueprints/BP_BaseCharacter.BPC_Health` _asbp_base_character) (`self.DamageAmount`))
            (`self.K2_DestroyActor`)))))))

(fn `UserConstructionScript`)