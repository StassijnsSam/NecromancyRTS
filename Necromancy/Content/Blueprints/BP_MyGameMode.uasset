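; Game mode Blueprint that tracks score, the villager win condition, level progression and player respawn.
; On BeginPlay it caches every villager, and CheckWin declares a win when each valid one is dead or tagged Zombie.
; Outside the Tutorial level, a win pauses the game, plays a fanfare and shows the win screen.
; OpenNextLevel only advances from Tutorial to Level01, and respawning reloads the current level.
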(event `Open Next Level`
  (bind _returnvalue (`GameplayStatics.GetCurrentLevelName` true))
  (if (`KismetStringLibrary.EqualEqual_StrStr` _returnvalue "Tutorial")
    (`GameplayStatics.OpenLevel` "Level01")))

(event `self.ReceiveBeginPlay`
  (`WidgetBlueprintLibrary.SetFocusToGameViewport`)
  ;[1 1 1] Get all the villagers so we can check win condition later
  (bind _outactors (`GameplayStatics.GetAllActorsOfClass` "/Game/Blueprints/BP_Villager.BP_Villager_C"))
  (set `self.Villagers` _outactors))

(event `RespawnPlayer`
  ;[1 1 1] Reload current level
  (bind _returnvalue (`GameplayStatics.GetCurrentLevelName` true))
  (`GameplayStatics.OpenLevel` (`KismetStringLibrary.Conv_StringToName` _returnvalue)))

(event `IncrementScore`
  (params (Amount :type Integer))
  ;[1 1 1] Add to score
  (set `self.Score` (+ Amount (`self.Score`))))

(event `CheckWin`
  (set `self.HasWon` true)
  (for _array_element (`self.Villagers`)
    (`/Engine/EditorBlueprintResources/StandardMacros.IsValid` _array_element
      (:`Is Valid`
        (if (not (or (`/Game/Blueprints/BPC_Health.IsDead` (`/Game/Blueprints/BP_BaseCharacter.BPC_Health` _array_element)) (`self.ActorHasTag` _array_element "Zombie")))
          ;[1 1 1] When one villager is still alive, you can break
          (set `self.HasWon` false)
          (break)))))
  (if (`self.HasWon`)
    ;[1 1 1] Dont show winscreen in tutorial
    (bind _returnvalue (`GameplayStatics.GetCurrentLevelName` true))
    (if (not (`KismetStringLibrary.EqualEqual_StrStr` _returnvalue "Tutorial"))
      (`GameplayStatics.SetGamePaused` true)
      ;[1 1 1] Win sound
      (`GameplayStatics.PlaySound2D` "/Game/Audio/source/success-fanfare-trumpets-6185.success-fanfare-trumpets-6185" 1.0 1.0 0.0 null null)
      ;[1 1 1] Show win screen
      (bind _returnvalue_2 (`|CreateWidget` "/Game/UI/BPW_WinScreen.BPW_WinScreen_C"))
      (`UserWidget.AddToViewport` _returnvalue_2 0))))

(fn `UserConstructionScript`)