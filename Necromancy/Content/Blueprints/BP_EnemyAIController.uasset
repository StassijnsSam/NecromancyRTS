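; AI controller for enemy villagers that runs BT_Enemy and targets actors tagged Friendly or Zombie through AI perception.
; Sensing a target sets line of sight and the enemy actor in the Blackboard; other perception updates start a timer that clears both on expiry.
; On possess it saves the start location, then waits a second for the weapon to spawn before storing its range for pathfinding.
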(event `self.AIPerception.OnTargetPerceptionUpdated`
  (params (Actor :type "Actor Object Reference") (Stimulus :type "AIStimulus Structure"))
  (bind _blackboard (`self.Blackboard`))
  (if (and (or (`self.ActorHasTag` Actor "Friendly") (`self.ActorHasTag` Actor "Zombie")) (`.bSuccessfullySensed` (break `AIStimulus` Stimulus)))
    ;[1 1 1] Clear the line of sight timer
    (`KismetSystemLibrary.K2_ClearAndInvalidateTimerHandle` (`self.EnemyTimer`))
    ;[1 1 1] Line of sight true
    (`BlackboardComponent.SetValueAsBool` _blackboard (`self.HasLineOfSight`) true)
    ;[1 1 1] Update target in blackboard
    (`BlackboardComponent.SetValueAsObject` _blackboard (`self.EnemyActor`) Actor)
    (else
      ;[1 1 1] Update line of sight to be false after timer runs out
      (bind _returnvalue (`KismetSystemLibrary.K2_SetTimerDelegate` (delegate `StartEnemyTimer`) (`self.LineOfSightTimer`)))
      (set `self.EnemyTimer` _returnvalue))))

(event `StartEnemyTimer`
  (bind _blackboard (`self.Blackboard`))
  ;[1 1 1] Update line of sight to be false after timer runs out
  (`BlackboardComponent.SetValueAsBool` _blackboard (`self.HasLineOfSight`) false)
  (`BlackboardComponent.SetValueAsObject` _blackboard (`self.EnemyActor`) null))

(event `self.ReceivePossess`
  (params (PossessedPawn :type "Pawn Object Reference"))
  (bind _blackboard (`self.Blackboard`))
  (`self.RunBehaviorTree` "/Game/AI/BT_Enemy.BT_Enemy")
  ;[1 1 1] Save start location to blackboard
  (`BlackboardComponent.SetValueAsVector` _blackboard (`self.Start Location`) (`self.K2_GetActorLocation` (`self.K2_GetPawn`)))
  ;[1 1 1] Need a delay so weapon is spawned in
  (`KismetSystemLibrary.Delay` 1.0)
  (bind _asbp_villager (cast `/Game/Blueprints/BP_Villager` (`self.K2_GetPawn`)))
  (bind _currentweapon (`/Game/Blueprints/BP_Villager.CurrentWeapon` _asbp_villager))
  ;[1 1 1] Save weapon range to Blackboard (used for pathfinding)
  (`/Engine/EditorBlueprintResources/StandardMacros.IsValid` _currentweapon
    (:`Is Valid`
      (`BlackboardComponent.SetValueAsFloat` _blackboard (`self.Range`) (`/Game/Blueprints/BP_BaseWeapon.Range` _currentweapon)))))

(fn `UserConstructionScript`)