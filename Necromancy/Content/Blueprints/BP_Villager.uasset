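; Villager character that fights with an attached weapon, dies into a physics body, and can be raised as an AI-controlled zombie.
; Weapon overlaps track targets by tag and allegiance, driving a looping damage timer.
; Health events update the bar and hit flicker; first death awards score and drops non-base weapons, while zombie death destroys it.
; As a zombie, its push zone breaks loose and launches moveable level objects, scoring by mass.
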(event `self.PushZone.OnComponentBeginOverlap`
  (params (OverlappedComponent :type "PrimitiveComponent Object Reference") (OtherActor :type "Actor Object Reference") (OtherComp :type "PrimitiveComponent Object Reference") (OtherBodyIndex :type Integer) (bFromSweep :type Boolean) (SweepResult :type "HitResult Structure (by ref)"))
  (bind (_returnvalue_x _returnvalue_y) (`KismetMathLibrary.BreakVector` (* (`KismetMathLibrary.Normal` (- (`self.K2_GetActorLocation` OtherActor) (`self.K2_GetActorLocation`))) 1000.0)))
  ;[1 1 1] Only works if you are a zombie
  (if (`self.ActorHasTag` "Zombie")
    ;[1 1 1] Only works on Moveable Level objects
    (if (`self.ActorHasTag` OtherActor "MoveableLevel")
      ;[1 1 1] If not yet simulating physics -> first time you touched it
      ; Play break sound
      ; Set simulate physics
      ; Add score
      (if (not (`SceneComponent.IsSimulatingPhysics` OtherComp "None"))
        (`GameplayStatics.SpawnSoundAttached` "/Game/Audio/Break.Break" OtherComp "None" (0.0 0.0 0.0) (struct) "KeepRelativeOffset" false 1.0 1.0 0.0 null null)
        (bind _asbp_my_game_mode (cast `/Game/Blueprints/BP_MyGameMode` (`GameplayStatics.GetGameMode`)))
        (`PrimitiveComponent.SetSimulatePhysics` OtherComp true)
        (`/Game/Blueprints/BP_MyGameMode.IncrementScore` _asbp_my_game_mode (`KismetMathLibrary.FCeil` (`PrimitiveComponent.GetMass` OtherComp))))
      (`PrimitiveComponent.AddImpulse` OtherComp (`KismetMathLibrary.MakeVector` _returnvalue_x _returnvalue_y 1000.0) "None" false))))

(event `self.BPC_Health.OnDamage`
  (`self.UpdateHealthBar`)
  (`self.Scream`)
  ;[1 1 1] Flicker material
  (`PrimitiveComponent.SetMaterial` (`self.Capsule`) 0 "/Game/StarterContent/Materials/M_Basic_Floor.M_Basic_Floor")
  (`KismetSystemLibrary.Delay` 0.1)
  (`PrimitiveComponent.SetMaterial` (`self.Capsule`) 0 (`self.OriginalMaterial`)))

(event `self.ReceiveBeginPlay`
  (bind _bpc_health (`self.BPC_Health`))
  (bind _currentweapon (`self.CurrentWeapon`))
  (bind _currentweapon_2 (`self.CurrentWeapon`))
  (`parent.ReceiveBeginPlay`)
  ;[1 1 1] Save original material (flor flickering)
  (set `self.OriginalMaterial` (`PrimitiveComponent.GetMaterial` (`self.Capsule`) 0))
  (`self.SpawnWeapon`)
  (`|ExecutionSequence`
    (:`then_0`
      ;[1 1 1] Bind to begin overlap event of weapon
      (`/Engine/EditorBlueprintResources/StandardMacros.IsValid` _currentweapon
        (:`Is Valid`
          (add `self.OnActorBeginOverlap` _currentweapon (delegate `WeaponOverlap`)))))
    (:`then_1`
      ;[1 1 1] Bind to end overlap event of weapon
      (`/Engine/EditorBlueprintResources/StandardMacros.IsValid` _currentweapon_2
        (:`Is Valid`
          (add `self.OnActorEndOverlap` _currentweapon_2 (delegate `EndWeaponOverlap`)))))
    (:`then_2`
      (if (`self.isDeadFromStart`)
        ;[1 1 1] Kill the enemy
        (set `self.ScoreOnKill` 0)
        (`/Game/Blueprints/BPC_Health.Do Damage` _bpc_health (`/Game/Blueprints/BPC_Health.CurrentHealth` _bpc_health))))))

(event `WeaponOverlap` :!signature `self.OnActorBeginOverlap`
  (params (OverlappedActor :type "Actor Object Reference") (OtherActor :type "Actor Object Reference"))
  (bind _nearbyenemies (`self.NearbyEnemies`))
  ;[1 1 1] Bind to begin overlap event of weapon
  (`/Engine/EditorBlueprintResources/StandardMacros.IsValid` OtherActor
    (:`Is Valid`
      (`|ExecutionSequence`
        (:`then_0`
          (if (or (`/Game/Blueprints/BPC_Health.IsDead` (`self.BPC_Health`)) (`self.ActorHasTag` OtherActor "Dead"))
            _
            (elif (`self.IsRaised`)
              ;[1 1 1] If raised, only enemies can be targets (no friendly fire)
              (if (`self.ActorHasTag` OtherActor "Enemy")
                ;[1 1 1] Clear invalid targets
                (for (_array_element _array_index) _nearbyenemies :!label _label
                  (`/Engine/EditorBlueprintResources/StandardMacros.IsValid` _array_element
                    (:`Is Not Valid`
                      (`KismetArrayLibrary.Array_Remove` _nearbyenemies _array_index))))
                ;[1 1 1] Set current enemy and start doing damage
                (`KismetArrayLibrary.Array_AddUnique` _nearbyenemies OtherActor)
                (set `self.CurrentEnemy` (`|GetArrayItem` (`self.NearbyEnemies`)))
                (`/Engine/EditorBlueprintResources/StandardMacros.IsValid` (`self.CurrentEnemy`)
                  (:`Is Valid`
                    _)
                  (:`Is Not Valid`
                    (set `self.CurrentEnemy` OtherActor)))
                (`KismetSystemLibrary.K2_SetTimer` null "DamageCurrentEnemyTarget" (`/Game/Blueprints/BP_BaseWeapon.AttackInterval` (`self.CurrentWeapon`)) true))
              (else
                ;[1 1 1] If not raised, only zombies and the player can be targets
                (if (or (`self.ActorHasTag` OtherActor "Zombie") (`self.ActorHasTag` OtherActor "Friendly"))
                  (goto _label))))))))))

(event `EndWeaponOverlap` :!signature `self.OnActorEndOverlap`
  (params (OverlappedActor :type "Actor Object Reference") (OtherActor :type "Actor Object Reference"))
  (bind _nearbyenemies (`self.NearbyEnemies`))
  ;[1 1 1] Bind to end overlap event of weapon
  ;[1 1 1] Remove from nearby enemies
  (`/Engine/EditorBlueprintResources/StandardMacros.IsValid` OtherActor
    (:`Is Valid`
      (if (`KismetArrayLibrary.Array_Contains` (`self.NearbyEnemies`) OtherActor)
        (`KismetArrayLibrary.Array_RemoveItem` (`self.NearbyEnemies`) OtherActor)
        ;[1 1 1] If it is the current enemy, clear damage timer and set new enemy as target
        (if (== OtherActor (`self.CurrentEnemy`))
          (`KismetSystemLibrary.K2_ClearTimer` null "DamageCurrentEnemyTarget")
          (if (> (`KismetArrayLibrary.Array_Length` _nearbyenemies) 0)
            (set `self.CurrentEnemy` (`|GetArrayItem` _nearbyenemies))
            (else
              (set `self.CurrentEnemy` null))))))))

(event `DamageCurrentEnemyTarget`
  (bind _nearbyenemies (`self.NearbyEnemies`))
  (bind _currentenemy (`self.CurrentEnemy`))
  (bind _currentenemy_2 (`self.CurrentEnemy`))
  (bind _returnvalue (`self.GetComponentByClass` _currentenemy_2 "/Game/Blueprints/BPC_Health.BPC_Health_C"))
  ;[1 1 1] Check if current enemy is alive
  (`/Engine/EditorBlueprintResources/StandardMacros.IsValid` _currentenemy_2
    (:`Is Valid`
      (`/Engine/EditorBlueprintResources/StandardMacros.IsValid` _returnvalue
        (:`Is Valid`
          (if (`/Game/Blueprints/BPC_Health.IsDead` (`self.BPC_Health`))
            ;[1 1 1] If you killed current target, remove it from the list and set the next target
            (`/Engine/EditorBlueprintResources/StandardMacros.IsValid` _currentenemy :!label _label_2
              (:`Is Valid`
                (`KismetArrayLibrary.Array_RemoveItem` (`self.NearbyEnemies`) _currentenemy)
                (`KismetSystemLibrary.K2_ClearTimer` null "DamageCurrentEnemyTarget")
                (if (> (`KismetArrayLibrary.Array_Length` _nearbyenemies) 0)
                  (set `self.CurrentEnemy` (`|GetArrayItem` _nearbyenemies))
                  (else
                    (set `self.CurrentEnemy` null)))))
            (else
              ;[1 1 1] Do damage and play audio based on weapontype
              (bind _iskilled (message `/Game/Blueprints/BPI_Damageable.Do Damage` _returnvalue (`/Game/Blueprints/BP_BaseWeapon.Damage` (`self.CurrentWeapon`))))
              (`AudioComponent.Play` (`/Game/Blueprints/BP_BaseWeapon.WeaponAudio` (`self.CurrentWeapon`)) 0.0)
              (if _iskilled
                (goto _label_2)))))))))

(event `self.BPC_Health.OnDead`
  ;[1 1 1] Check if you won
  (bind _asbp_my_game_mode (cast `/Game/Blueprints/BP_MyGameMode` (`GameplayStatics.GetGameMode`)))
  (`/Game/Blueprints/BP_MyGameMode.CheckWin` _asbp_my_game_mode)
  ;[1 1 1] If a raised enemy dies its dead for good
  (if (`self.IsRaised`)
    ;[1 1 1] Destroy attached actors and itself
    (for _array_element (`self.GetAttachedActors` self true)
      (`/Engine/EditorBlueprintResources/StandardMacros.IsValid` _array_element
        (:`Is Valid`
          (`self.K2_DestroyActor` _array_element))))
    (`self.K2_DestroyActor`)
    (else
      (`self.Die`)
      (`self.UpdateHealthBar`)
      ;[1 1 1] Add score
      (bind _asbp_my_game_mode_2 (cast `/Game/Blueprints/BP_MyGameMode` (`GameplayStatics.GetGameMode`)))
      (`/Game/Blueprints/BP_MyGameMode.IncrementScore` _asbp_my_game_mode_2 (`self.ScoreOnKill`))
      (`self.UpdateWeaponOnDeath`)
      ;[1 1 1] Clear all current nearby enemies!
      ; Important, otherwise you can have wrong enemies in there
      (`KismetArrayLibrary.Array_Clear` (`self.NearbyEnemies`)))))

(fn `ChangeMaterial`
  (params (Material :type "MaterialInstance Object Reference"))
  (`PrimitiveComponent.SetMaterial` (`self.RightHand`) 0 Material)
  (`PrimitiveComponent.SetMaterial` (`self.LeftHand`) 0 Material)
  (`PrimitiveComponent.SetMaterial` (`self.Capsule`) 0 Material))

(fn `Die`
  ;[1 1 1] get rid of controller
  ; This is needed instead of unpossess since otherwise the old controller can not be deleted
  (`self.DetachFromControllerPendingDestroy`)
  ;[1 1 1] Set tag to Dead
  (set `self.Tags` (`self.DeadTag`))
  ;[1 1 1] Give enemy the dead material
  (`self.ChangeMaterial` "/Game/Materials/MI_Dead.MI_Dead")
  (set `self.OriginalMaterial` "/Game/Materials/MI_Dead.MI_Dead")
  (`PrimitiveComponent.SetSimulatePhysics` (`self.CapsuleComponent`) true))

(fn `Raise`
  (locals (newTags :type "Array of Name") (ZombieAIClass :type "Actor Class Reference" :default "BlueprintGeneratedClass'/Game/Blueprints/BP_ZombieAIController.BP_ZombieAIController_C'"))
  (bind (_returnvalue_location _returnvalue_rotation) (`KismetMathLibrary.BreakTransform` (`self.GetTransform` (`GameplayStatics.GetPlayerPawn` 0))))
  (`self.ChangeMaterial` "/Game/Materials/MI_Zombie.MI_Zombie")
  (set `self.OriginalMaterial` "/Game/Materials/MI_Zombie.MI_Zombie")
  (set `self.Tags` (`local.newTags`))
  (set `self.IsRaised` true)
  (`PrimitiveComponent.SetSimulatePhysics` (`self.CapsuleComponent`) false)
  (`self.K2_SetActorRotation` _returnvalue_rotation)
  (`/Game/Blueprints/BPC_Health.ResetHealth` (`self.BPC_Health`))
  (set `CharacterMovementComponent.MaxWalkSpeed` 400.0 (`self.CharacterMovement`))
  (bind _returnvalue (`|SpawnActorFromClass` (`local.ZombieAIClass`) (`KismetMathLibrary.MakeTransform` (0.0 0.0 0.0)) "Undefined" "OverrideRootScale" null null))
  (bind _asbp_zombie_aicontroller (cast `/Game/Blueprints/BP_ZombieAIController` _returnvalue))
  (`Controller.Possess` _asbp_zombie_aicontroller self)
  ;[1 1 1] Start the zombie noises
  (`AudioComponent.Play` (`self.ZombieNoises`) 0.0))

(fn `Scream`
  ;[1 1 1] Only living enemies scream when taking damage
  (if (not (or (`self.ActorHasTag` "Dead") (`self.ActorHasTag` "Zombie")))
    (`AudioComponent.Play` (`self.Hurt`) 0.0)))

(fn `SpawnWeapon`
  (bind _returnvalue (`|SpawnActorFromClass` (`self.WeaponClass`) (`SceneComponent.K2_GetComponentToWorld` (`self.WeaponSocket`)) "Undefined" "OverrideRootScale" null null))
  (set `self.CurrentWeapon` _returnvalue)
  (`self.K2_AttachToComponent` _returnvalue (`self.WeaponSocket`) "None" "SnapToTarget" "SnapToTarget" "KeepRelative" true))

(fn `UpdateHealthBar`
  (bind _asbpw_enemy_health_bar (cast `/Game/UI/BPW_EnemyHealthBar` (`WidgetComponent.GetUserWidgetObject` (`self.Health Bar`))))
  (set `/Game/UI/BPW_EnemyHealthBar.HealthPercentage` (`/Game/Blueprints/BPC_Health.GetHealthPercentage` (`self.BPC_Health`)) _asbpw_enemy_health_bar))

(fn `UpdateWalkSpeed`
  (params (WalkSpeed :type "Float (double-precision)"))
  (set `CharacterMovementComponent.MaxWalkSpeed` WalkSpeed (`self.CharacterMovement`)))

(fn `UpdateWeaponOnDeath`
  (bind _currentweapon (`self.CurrentWeapon`))
  (`/Engine/EditorBlueprintResources/StandardMacros.IsValid` _currentweapon
    (:`Is Valid`
      (if (not (== (`GameplayStatics.GetObjectClass` _currentweapon) "/Game/Blueprints/BP_BaseWeapon.BP_BaseWeapon_C"))
        (`self.K2_DetachFromActor` _currentweapon "KeepWorld" "KeepWorld" "KeepRelative")
        (`PrimitiveComponent.SetSimulatePhysics` (`/Game/Blueprints/BP_Spear.StaticMesh` _currentweapon) true)
        (bind _returnvalue (`|SpawnActorFromClass` "/Game/Blueprints/BP_BaseWeapon.BP_BaseWeapon_C" (`SceneComponent.K2_GetComponentToWorld` (`self.WeaponSocket`)) "Undefined" "OverrideRootScale" null null))
        (set `self.CurrentWeapon` _returnvalue)
        (`self.K2_AttachToComponent` _returnvalue (`self.WeaponSocket`) "None" "SnapToTarget" "SnapToTarget" "KeepRelative" true)))))

(fn `UserConstructionScript`
  (`parent.UserConstructionScript`)
  (if (`self.isDeadFromStart`)
    (`self.ChangeMaterial` "/Game/Materials/MI_Dead.MI_Dead")))