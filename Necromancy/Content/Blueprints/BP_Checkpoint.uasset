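; BP_Checkpoint is a checkpoint actor, apparently for a tutorial level, that drives a linked BP_Ghost and chains to the next checkpoint.
; When the player enters a checkpoint that can start, it disarms itself, reveals its ghost and starts it; leaving the box completes a finished, auto-disappearing ghost.
; ActivateNext either opens the next level via the game mode or arms the next checkpoint, reveals its ghost and retargets the tutorial arrow to it.
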(event `self.ReceiveActorBeginOverlap`
  (params (OtherActor :type "Actor Object Reference"))
  (bind _ghost (`self.Ghost`))
  ;[1 1 1] Start the ghost when walking into a checkpoint that can start
  (cast `/Game/Blueprints/BP_PlayerCharacter` OtherActor)
  (if (`self.CanStart`)
    (set `self.CanStart` false)
    (`/Engine/EditorBlueprintResources/StandardMacros.IsValid` _ghost
      (:`Is Valid`
        (`self.SetActorHiddenInGame` _ghost false)
        (bind _asbp_ghost (cast `/Game/Blueprints/BP_Ghost` _ghost))
        (`/Game/Blueprints/BP_Ghost.StartGhost` _asbp_ghost)))))

(event `ActivateNext`
  (bind _nextcheckpoint (`self.NextCheckPoint`))
  (if (`self.IsFinishLevel`)
    ;[1 1 1] If the checkpoint is the last of the tutorial level, open next level
    (bind _asbp_my_game_mode (cast `/Game/Blueprints/BP_MyGameMode` (`GameplayStatics.GetGameMode`)))
    (`/Game/Blueprints/BP_MyGameMode.Open Next Level` _asbp_my_game_mode)
    (else
      ;[1 1 1] Set next checkpoint to be able to start
      (`/Engine/EditorBlueprintResources/StandardMacros.IsValid` _nextcheckpoint
        (:`Is Valid`
          (bind _asbp_checkpoint (cast `/Game/Blueprints/BP_Checkpoint` _nextcheckpoint))
          (set `/Game/Blueprints/BP_Checkpoint.CanStart` true _asbp_checkpoint)
          (bind _ghost (`/Game/Blueprints/BP_Checkpoint.Ghost` _asbp_checkpoint))
          ;[1 1 1] Set ghost visible
          (`/Engine/EditorBlueprintResources/StandardMacros.IsValid` _ghost
            (:`Is Valid`
              (`self.SetActorHiddenInGame` _ghost false)
              ;[1 1 1] Set new ghost as tutorial arrow target
              (bind _returnvalue (`GameplayStatics.GetActorOfClass` "/Game/Blueprints/BP_TutorialArrow.BP_TutorialArrow_C"))
              (`/Engine/EditorBlueprintResources/StandardMacros.IsValid` _returnvalue
                (:`Is Valid`
                  (bind _ghost_2 (`/Game/Blueprints/BP_Checkpoint.Ghost` _asbp_checkpoint))
                  (`/Engine/EditorBlueprintResources/StandardMacros.IsValid` _ghost_2
                    (:`Is Valid`
                      (set `/Game/Blueprints/BP_TutorialArrow.CurrentTarget` _ghost_2 _returnvalue))))))))))))

(event `self.Box.OnComponentEndOverlap`
  (params (OverlappedComponent :type "PrimitiveComponent Object Reference") (OtherActor :type "Actor Object Reference") (OtherComp :type "PrimitiveComponent Object Reference") (OtherBodyIndex :type Integer))
  (bind _ghost (`self.Ghost`))
  ;[1 1 1] When you walk out and the ghost is finished, destroy the ghost
  (cast `/Game/Blueprints/BP_PlayerCharacter` OtherActor)
  (`/Engine/EditorBlueprintResources/StandardMacros.IsValid` _ghost
    (:`Is Valid`
      (bind _asbp_ghost (cast `/Game/Blueprints/BP_Ghost` _ghost))
      (if (`/Game/Blueprints/BP_Ghost.Completed` _asbp_ghost)
        (if (`/Game/Blueprints/BP_Ghost.IsAutoDisappear` _asbp_ghost)
          (`/Game/Blueprints/BP_Ghost.CompleteGhost` _asbp_ghost))))))

(fn `UserConstructionScript`)