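; BP_PlayerCharacter is the player character, handling zombie knockback, damage and heal feedback, and death.
; Overlapping its PushZone launches BP_Villager actors tagged "Zombie" away from the player with a velocity-change impulse plus slight lift.
; BPC_Health events drive the rest: damage plays a sound and briefly swaps the mesh material, and healing plays a sound.
; On death it asks BP_MyGameMode to respawn the player, then destroys itself.
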(event `self.ReceiveBeginPlay`
  (`parent.ReceiveBeginPlay`))

(event `self.PushZone.OnComponentBeginOverlap`
  (params (OverlappedComponent :type "PrimitiveComponent Object Reference") (OtherActor :type "Actor Object Reference") (OtherComp :type "PrimitiveComponent Object Reference") (OtherBodyIndex :type Integer) (bFromSweep :type Boolean) (SweepResult :type "HitResult Structure (by ref)"))
  (bind (_returnvalue_x _returnvalue_y) (`KismetMathLibrary.BreakVector` (* (- (`self.K2_GetActorLocation` OtherActor) (`self.K2_GetActorLocation`)) 0.8)))
  (`/Engine/EditorBlueprintResources/StandardMacros.IsValid` OtherActor
    (:`Is Valid`
      (if (`self.ActorHasTag` OtherActor "Zombie")
        (bind _asbp_villager (cast `/Game/Blueprints/BP_Villager` OtherActor))
        ;[1 1 1] Push zombie away
        (`CharacterMovementComponent.AddImpulse` (`Character.CharacterMovement` _asbp_villager) (`KismetMathLibrary.MakeVector` _returnvalue_x _returnvalue_y 30.0) true)))))

(event `self.BPC_Health.OnDead`
  ;[1 1 1] Remove player and reload level when you die
  (bind _asbp_my_game_mode (cast `/Game/Blueprints/BP_MyGameMode` (`GameplayStatics.GetGameMode`))
    (:`then`
      (`/Game/Blueprints/BP_MyGameMode.RespawnPlayer` _asbp_my_game_mode))
    (:`CastFailed`
      _))
  (`self.K2_DestroyActor`))

(event `self.BPC_Health.OnDamage`
  (bind _staticmesh (`self.StaticMesh`))
  ;[1 1 1] Hurt sound
  (`GameplayStatics.SpawnSoundAttached` "/Game/Audio/Hurt.Hurt" (`self.Mesh`) "None" (0.0 0.0 0.0) (struct) "KeepRelativeOffset" false 1.0 1.0 0.0 null null)
  ;[1 1 1] Material flicker
  (set `self.OldMaterial` (`PrimitiveComponent.GetMaterial` _staticmesh 0))
  (`PrimitiveComponent.SetMaterial` _staticmesh 0 "/Game/StarterContent/Materials/M_Basic_Floor.M_Basic_Floor")
  (`KismetSystemLibrary.Delay` 0.15)
  (`PrimitiveComponent.SetMaterial` (`self.StaticMesh`) 0 (`self.OldMaterial`)))

(event `self.BPC_Health.OnHeal`
  ;[1 1 1] Heal sound
  (`GameplayStatics.SpawnSoundAttached` "/Game/Audio/Heal.Heal" (`self.StaticMesh`) "None" (0.0 0.0 0.0) (struct) "KeepRelativeOffset" false 1.0 1.0 0.0 null null))

(fn `UserConstructionScript`
  (`parent.UserConstructionScript`))