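; AI controller for a zombie pawn that follows the player, moves to a position or attacks an enemy.
; A looping half-second timer started on BeginPlay runs Behavior, which switches on CurrentBehaviorType and reissues the matching AI MoveTo.
; The attack branch calls CallAttack as soon as the move toward Enemy is issued, without waiting for arrival.
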(event `self.ReceiveBeginPlay`
  ;[1 1 1] Check to change behavior every 0.5s
  (`KismetSystemLibrary.K2_SetTimer` null "Behavior" 0.5 true))

(event `Behavior`
  (switch `string` (`self.CurrentBehaviorType`)
    (:`Follow`
      ;[1 1 1] Follow player
      (`|AIMoveTo` (`self.K2_GetPawn`) (0.0 0.0 0.0) (`GameplayStatics.GetPlayerCharacter` 0) 30.0))
    (:`MoveToPos`
      ;[1 1 1] Move to location
      (`|AIMoveTo` (`self.K2_GetPawn`) (`self.MoveTo`) null 5.0 true))
    (:`AttackOnPos`
      ;[1 1 1] Move to enemy to attack
      (`|AIMoveTo` (`self.K2_GetPawn`) (0.0 0.0 0.0) (`self.Enemy`) 5.0 true
        (:`then`
          (`self.Attack`))))))

(fn `UserConstructionScript`)