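; Health component that tracks current and max health for its owner and resets to full on BeginPlay.
; DoDamage clamps health between zero and max, treats negative amounts as healing, and returns whether health is zero.
; It fires OnHeal for negative amounts, OnDead when a hit reduces health to zero, and OnDamage otherwise, including hits on an already-dead owner.
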(event `ResetHealth`
  ;[1 1 1] Reset health to max
  (set `self.CurrentHealth` (`self.MaxHealth`)))

(event `self.ReceiveBeginPlay`
  (`self.ResetHealth`))

(fn `Do Damage`
  (params (Amount :type "Float (double-precision)"))
  (returns (IsKilled :type Boolean))
  (locals (OriginalHealth :type "Float (double-precision)"))
  (bind _isdead (`self.IsDead`))
  ;[1 1 1] Cache original health value
  (set `local.OriginalHealth` (`self.CurrentHealth`))
  (bind _output_get (set `self.CurrentHealth` (`KismetMathLibrary.FClamp` (- (`self.CurrentHealth`) Amount) 0.0 (`self.MaxHealth`))))
  ;[1 1 1] Was this a heal?
  (if (< Amount 0.0)
    (`self.OnHeal`)
    (elif (and _isdead (> (`local.OriginalHealth`) _output_get))
      (`self.OnDead`)
      (else
        (`self.OnDamage`))))
  (return _isdead))

(fn `GetHealthPercentage`
  (returns (HealthPercentage :type "Float (double-precision)"))
  (return (/ (`self.CurrentHealth`) (`self.MaxHealth`))))

(fn `IsDead`
  (returns (IsDead :type Boolean))
  (return (== (`self.GetHealthPercentage`) 0.0)))