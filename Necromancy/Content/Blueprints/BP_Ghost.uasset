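; Ghost actor that shows a timed sequence of messages on a text widget, then completes by activating the next checkpoint and destroying itself.
; StartGhost begins the timer-driven text loop.
; Player overlap, or text end with IsAutoDisappear, checks that villagers are dead or zombies, then game mode score against ScoreLimit.
; The score check overwrites the villager result in Completed, and completion also requires finished text.
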(event `UpdateText`
  ;[1 1 1] Loop over strings
  (`self.SetText`)
  (if (< (+ (`self.CurrentIndex`) 1) (`KismetArrayLibrary.Array_Length` (`self.TextArray`)))
    (set `self.CurrentIndex` (+ (`self.CurrentIndex`) 1))
    (else
      ;[1 1 1] Set text to complete and check requirements
      (`KismetSystemLibrary.K2_ClearTimer` null "UpdateText")
      (set `self.TextCompleted` true)
      (if (`self.IsAutoDisappear`)
        (`self.Check Requirements`)))))

(event `StartGhost`
  ;[1 1 1] Set text wdiget visible and display first string
  (`SceneComponent.SetVisibility` (`self.TextWidget`) true true)
  (`self.SetText`)
  (if (< (`self.CurrentIndex`) (`KismetArrayLibrary.Array_Length` (`self.TextArray`)))
    (set `self.CurrentIndex` (+ (`self.CurrentIndex`) 1))
    ;[1 1 1] Loop over strings
    (`KismetSystemLibrary.K2_SetTimerDelegate` (delegate `UpdateText`) (`self.TextDelay`) true)))

(event `CompleteGhost`
  (bind _checkpoint (`self.CheckPoint`))
  ;[1 1 1] Destroy ghost and activate next checkpoint
  (`/Engine/EditorBlueprintResources/StandardMacros.IsValid` _checkpoint
    (:`Is Valid`
      (bind _asbp_checkpoint (cast `/Game/Blueprints/BP_Checkpoint` _checkpoint))
      (`/Game/Blueprints/BP_Checkpoint.ActivateNext` _asbp_checkpoint))
    (:`Is Not Valid`
      _))
  (`self.K2_DestroyActor`))

(event `self.CapsuleComponent.OnComponentBeginOverlap`
  (params (OverlappedComponent :type "PrimitiveComponent Object Reference") (OtherActor :type "Actor Object Reference") (OtherComp :type "PrimitiveComponent Object Reference") (OtherBodyIndex :type Integer) (bFromSweep :type Boolean) (SweepResult :type "HitResult Structure (by ref)"))
  ;[1 1 1] Check requirements for ghost completion
  (cast `/Game/Blueprints/BP_PlayerCharacter` OtherActor)
  (`self.CheckActorsDeath` :!label _label)
  (`self.CheckScore`)
  (if (and (`self.Completed`) (`self.TextCompleted`))
    (`self.CompleteGhost`)))

(event `Check Requirements`
  ;[1 1 1] Check requirements for ghost completion
  (goto _label))

(event `CheckActorsDeath`
  (for _array_element (`self.Villagers`)
    (`/Engine/EditorBlueprintResources/StandardMacros.IsValid` _array_element
      (:`Is Valid`
        (bind _asbp_villager (cast `/Game/Blueprints/BP_Villager` _array_element))
        (if (or (`/Game/Blueprints/BPC_Health.IsDead` (`/Game/Blueprints/BP_BaseCharacter.BPC_Health` _asbp_villager)) (`self.ActorHasTag` _asbp_villager "Zombie"))
          (set `self.IsDead` true)
          (else
            ;[1 1 1] When you find a living one, you can break the loop
            (set `self.IsDead` false)
            (break))))
      (:`Is Not Valid`
        ;[1 1 1] If all are dead, set completed to true
        (set `self.Completed` true :!label _label_2))))
  (if (`self.IsDead`)
    (goto _label_2)))

(event `CheckScore`
  (bind _asbp_my_game_mode (cast `/Game/Blueprints/BP_MyGameMode` (`GameplayStatics.GetGameMode`)))
  ;[1 1 1] Check if current score is higher than score requirement
  (set `self.Completed` (>= (`/Game/Blueprints/BP_MyGameMode.Score` _asbp_my_game_mode) (`self.ScoreLimit`))))

(fn `ChangeMaterial`
  (params (Material :type "MaterialInstance Object Reference"))
  (`PrimitiveComponent.SetMaterial` (`self.RightHand`) 0 Material)
  (`PrimitiveComponent.SetMaterial` (`self.LeftHand`) 0 Material)
  (`PrimitiveComponent.SetMaterial` (`self.Capsule`) 0 Material))

(fn `SetText`
  (bind _asbpw_text (cast `/Game/UI/BPW_Text` (`WidgetComponent.GetUserWidgetObject` (`self.TextWidget`))))
  (set `/Game/UI/BPW_Text.text` (`KismetTextLibrary.Conv_StringToText` (`|GetArrayItem` (`self.TextArray`) (`self.CurrentIndex`))) _asbpw_text))

(fn `UserConstructionScript`)